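; Interactable note pickup Blueprint that adds a journal entry and shows the note on screen when the player interacts with it.
; On interact, it looks up its NoteID in the game mode's note database and, if found, passes the entry to the player controller's journal.
; It then creates the note widget, fills in the body text and prints a confirmation message.
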(event EventBeginPlay)

(event Collision|EventActorBeginOverlap
  (params (OtherActor :type Actor%20Object%20Reference)))

(event EventTick
  (params (DeltaSeconds :type Float%20%28single-precision%29)))

(event EventOnInteract
  (params (Caller :type Pawn%20Object%20Reference))
  (bind _returnvalue (Game|GetPlayerController 0))
  (|CallParentFunction Caller)
  (bind _asimpbase_game_mode (Utilities|Casting|CastToIMPBaseGameMode (Game|GetGameMode)))
  (bind (_outentry _returnvalue_2) (Class|IMPBaseGameMode|GetNoteEntryfromDB _asimpbase_game_mode (Variables|Default|GetNoteID)))
  (if _returnvalue_2
    (bind _asimpplayer_controller (Utilities|Casting|CastToIMPPlayerController _returnvalue))
    (Class|IMPPlayerController|AddNewJournalEntry _asimpplayer_controller _outentry)
    (bind _returnvalue_3 (UserInterface|CreateWidget "/Game/DemoContent/Assets/DEV_NotePickup/NotePickup_dev/NoteWidget.NoteWidget_C" _returnvalue))
    (UserInterface|Viewport|AddtoViewport _returnvalue_3 0)
    (Rendering|Components|TextRender|SetText (Variables|/Game/DemoContent/Assets/DEV_NotePickup/NotePickup_dev/NoteWidget.NoteWidget_C|GetNote_Body _returnvalue_3) (.NoteBody (Utilities|Struct|BreakIMPNoteEntry _outentry)))
    (Development|PrintString "Journal Entry Added. Open Player Menu to check your Journal")))

(fn ConstructionScript)