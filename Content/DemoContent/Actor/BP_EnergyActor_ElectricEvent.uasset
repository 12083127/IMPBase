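; BP_EnergyActor_ElectricEvent is a demo energy actor that reacts when it is drained by affecting a linked sconce.
; Its drained event runs the parent logic, then, if the sconce reference is valid, sets that sconce's PointLight2 intensity to zero and spawns an explosion particle emitter at its location.
; The construction script only calls the parent, and the other default events are disabled.
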(event EventBeginPlay
  (|CallParentFunction) ; This node is disabled and will not be called.\nDrag off pins to build functionality.
)

(event Collision|EventActorBeginOverlap
  (params (OtherActor :type Actor%20Object%20Reference))
  (|CallParentFunction OtherActor) ; This node is disabled and will not be called.\nDrag off pins to build functionality.
)

(event EventTick
  (params (DeltaSeconds :type Float%20%28single-precision%29))
  (|CallParentFunction DeltaSeconds) ; This node is disabled and will not be called.\nDrag off pins to build functionality.
)

(event EventOnDrainedEvent
  (bind _sconceref (Variables|Default|GetSconceRef))
  (|CallParentFunction)
  (if (Utilities|IsValid (Variables|Default|GetSconceRef))
    (Rendering|Components|Light|SetIntensity (Variables|/Game/StarterContent/Blueprints/Blueprint_WallSconce.Blueprint_WallSconce_C|GetPointLight2 _sconceref) 0.0)
    (Effects|SpawnEmitteratLocation "/Game/StarterContent/Particles/P_Explosion.P_Explosion" (Transformation|GetActorLocation _sconceref))))

(fn ConstructionScript
  (|CallParentFunction))