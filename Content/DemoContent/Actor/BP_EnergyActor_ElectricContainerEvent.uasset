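; BP_EnergyActor_ElectricContainerEvent is a child energy actor, apparently an electric container, that gives visual feedback on a linked sconce when charged.
; It overrides OnChargedEvent, calls the parent logic, then turns the PointLight2 of SconceRef green if that reference is valid.
; All other behavior comes from the parent class, as the construction script only calls its parent and the remaining event stubs are disabled.
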(event EventBeginPlay
  (|CallParentFunction) ; This node is disabled and will not be called.\nDrag off pins to build functionality.
)

(event Collision|EventActorBeginOverlap
  (params (OtherActor :type Actor%20Object%20Reference))
  (|CallParentFunction OtherActor) ; This node is disabled and will not be called.\nDrag off pins to build functionality.
)

(event EventTick
  (params (DeltaSeconds :type Float%20%28single-precision%29))
  (|CallParentFunction DeltaSeconds) ; This node is disabled and will not be called.\nDrag off pins to build functionality.
)

(event EventOnChargedEvent
  (|CallParentFunction)
  (if (Utilities|IsValid (Variables|Default|GetSconceRef))
    (Rendering|Components|Light|SetLightColor (Variables|/Game/StarterContent/Blueprints/Blueprint_WallSconce.Blueprint_WallSconce_C|GetPointLight2 (Variables|Default|GetSconceRef)) "(R=0.000000,G=0.859375,B=0.115257,A=1.000000)" true)))

(fn ConstructionScript
  (|CallParentFunction))