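; Master inventory preview actor that displays the active item's static mesh, with the mesh component set tickable while paused.
; UpdatePreviewMesh swaps in the mesh and resets its transform and pivot rotation when the item's instance and ID both differ from the last seen.
; AdjustPreviewMeshScale then fits the largest bounds extent to the preview frame and offsets the mesh by its local bounds center.
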(event EventBeginPlay
  (Class|ActorComponent|SetTickablewhenPaused (Variables|Default|GetPreviewMesh) true))

(event Collision|EventActorBeginOverlap
  (params (OtherActor :type Actor%20Object%20Reference)))

(event EventTick
  (params (DeltaSeconds :type Float%20%28single-precision%29)))

(event EventUpdatePreviewMesh
  (params (ActiveItem :type IMP%20Inventory%20Item%20Base%20Object%20Reference))
  (bind _previewmesh (Variables|Default|GetPreviewMesh))
  (if (Utilities|IsValid ActiveItem)
    (Variables|Default|SetItem ActiveItem)
    (if (Utilities|IsValid (Variables|Default|GetLastSeenItem))
      (if (and (!= (Variables|Default|GetLastSeenItem) (Variables|Default|GetItem)) (Utilities|Name|NotEqual(Name) (Variables|/Script/IMPBase.IMPInventoryItemBase|GetItemID (Variables|Default|GetLastSeenItem)) (Variables|/Script/IMPBase.IMPInventoryItemBase|GetItemID (Variables|Default|GetItem))))
        (Variables|Default|SetLastSeenItem (Variables|Default|GetItem) :!label _label)
        (Components|StaticMesh|SetStaticMesh _previewmesh (Variables|/Script/IMPBase.IMPInventoryItemBase|GetItemMesh (Variables|Default|GetItem)))
        (Transformation|SetWorldScale3D _previewmesh "1.000000,1.000000,1.000000")
        (Transformation|SetRelativeLocation _previewmesh "0, 0, 0" false true)
        (Transformation|SetRelativeRotation (Variables|Default|GetRotationPivot) "0, 0, 0" false false)
        (CallFunction|AdjustPreviewMeshScale))
      (else
        (goto _label)))))

(fn ConstructionScript)

(fn GetPreviewMeshMaxExtends
  (bind _previewmesh (Variables|Default|GetPreviewMesh))
  (bind _boxextent (Collision|GetComponentBounds _previewmesh))
  (bind (_x _y _z) (Math|Vector|BreakVector _boxextent))
  (return (Math|Float|Max(Float) _x _y _z)))

(fn AdjustPreviewMeshScale
  (bind _previewmesh (Variables|Default|GetPreviewMesh))
  (bind _previewmesh_2 (Variables|Default|GetPreviewMesh))
  (bind (_min _max) (Components|StaticMesh|GetLocalBounds _previewmesh))
  (if (== (CallFunction|GetPreviewMeshMaxExtends) 0.0)
    (LocalVariables|SetScalar 1.0)
    (else
      (LocalVariables|SetScalar (/ (Class|IMPPreviewCaptureBase|GetPreviewFrameExtends) (CallFunction|GetPreviewMeshMaxExtends)))))
  (Transformation|SetWorldScale3D _previewmesh_2 (* (Transformation|GetWorldScale _previewmesh_2) (LocalVariables|GetScalar)))
  (Transformation|AddRelativeLocation (Variables|Default|GetPreviewMesh) (- (Variables|/Script/Engine.SceneComponent|GetRelativeLocation _previewmesh) (/ (+ _min _max) 2.0)) false false)
  (return))