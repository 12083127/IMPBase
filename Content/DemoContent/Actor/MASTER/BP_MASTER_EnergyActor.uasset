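; BP_MASTER_EnergyActor is a master demo actor whose mesh materials visualize the type and charge of its energy component.
; The construction script picks a color from a color struct by the component's energy type, with None falling back to the electric color.
; BeginPlay pushes that color and a glow multiplier to the mesh materials, and Tick updates their energy level from the component's normalized value every frame.
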(event EventBeginPlay
  (|CallParentFunction)
  (Rendering|Material|SetVectorParameterValueonMaterials (Variables|Character|GetMesh) "HighEnergyColor" (Math|Conversions|ToVector(LinearColor) (Variables|Default|GetEnergyColor)))
  (Rendering|Material|SetScalarParameterValueonMaterials (Variables|Character|GetMesh) "GlowMulitplier" (Variables|IMPBase|GetGlowMultiplier)))

(event Collision|EventActorBeginOverlap
  (params (OtherActor :type Actor%20Object%20Reference)))

(event EventTick
  (params (DeltaSeconds :type Float%20%28single-precision%29))
  (|CallParentFunction DeltaSeconds)
  (Rendering|Material|SetScalarParameterValueonMaterials (Variables|Character|GetMesh) "EnergyLevel" (Class|IMPEnergyComponent|GetEnergyLevelNormalized (Variables|Default|GetEnergyComponent))))

(fn ConstructionScript
  (bind _energycolorstruct (LocalVariables|GetEnergyColorStruct))
  (switch Utilities|FlowControl|Switch|SwitchonEEnergyType (Class|IMPEnergyComponent|GetEnergyType (Variables|Default|GetEnergyComponent))
    (:ET_None
      (Variables|Default|SetEnergyColor (.electricenergycolor _energycolorstruct) :!label _label))
    (:ET_Electric
      (goto _label))
    (:ET_Fire
      (Variables|Default|SetEnergyColor (.fireenergycolor _energycolorstruct)))
    (:ET_Water
      (Variables|Default|SetEnergyColor (.waterenergycolor _energycolorstruct)))))