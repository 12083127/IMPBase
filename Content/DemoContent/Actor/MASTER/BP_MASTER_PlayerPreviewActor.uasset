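; Preview actor that shows a copy of the player character's skeletal mesh, set to keep animating while the game is paused.
; UpdatePreviewMesh copies the mesh and materials from BP_IMPPlayer, resets the transform and loops a third-person idle animation.
; It then scales the mesh by the ratio of frame extent to largest bounds extent and lowers it by the resulting extent to fit differently sized characters.
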(event EventBeginPlay
  (Class|ActorComponent|SetTickablewhenPaused (Variables|Default|GetPlayerPreview) true))

(event Collision|EventActorBeginOverlap
  (params (OtherActor :type Actor%20Object%20Reference)))

(event EventTick
  (params (DeltaSeconds :type Float%20%28single-precision%29)))

(event EventUpdatePreviewMesh
  (params (ActiveItem :type IMP%20Inventory%20Item%20Base%20Object%20Reference))
  (bind _asbp_impplayer (Utilities|Casting|CastToBP_IMPPlayer (Game|GetPlayerCharacter 0)))
  (Transformation|SetRelativeLocation (Variables|Default|GetPlayerPreview) "0, 0, 0" false true)
  (Transformation|SetRelativeScale3D (Variables|Default|GetPlayerPreview) "1.000000,1.000000,1.000000")
  (Class|SkinnedMeshComponent|SetSkeletalMesh (Variables|Default|GetPlayerPreview) (Variables|/Script/Engine.SkinnedMeshComponent|GetSkeletalMesh (Default|GetSkeletalMeshComponent _asbp_impplayer)) true)
  (for (_array_element _array_index) (Rendering|Material|GetMaterials (Default|GetSkeletalMeshComponent _asbp_impplayer))
    (Rendering|Material|SetMaterial (Variables|Default|GetPlayerPreview) _array_index _array_element))
  (Components|Animation|PlayAnimation (Variables|Default|GetPlayerPreview) "/Game/Mannequin/Animations/ThirdPersonIdle.ThirdPersonIdle" true)
  (CallFunction|AdjustPreviewMeshScale))

(fn ConstructionScript)

(fn GetPreviewMeshMaxExtends
  (return (Math|Vector|GetMaxElement (.BoxExtent (Collision|GetComponentBounds (Variables|Default|GetPlayerPreview))))))

(fn AdjustPreviewMeshScale
  (bind _maxextends (CallFunction|GetPreviewMeshMaxExtends))
  (bind _playerpreview (Variables|Default|GetPlayerPreview))
  (if (== _maxextends 0.0)
    (LocalVariables|SetScalar 1.0)
    (else
      (LocalVariables|SetScalar (/ (Class|IMPPreviewCaptureBase|GetPreviewFrameExtends) _maxextends))))
  (Transformation|SetWorldScale3D _playerpreview (* (Transformation|GetWorldScale _playerpreview) (LocalVariables|GetScalar)))
  (Transformation|AddRelativeLocation (Variables|Default|GetPlayerPreview) (- (Variables|/Script/Engine.SceneComponent|GetRelativeLocation (Variables|Default|GetPlayerPreview)) (Math|Vector|MakeVector 0.0 0.0 (CallFunction|GetPreviewMeshMaxExtends))) false true)
  (return))