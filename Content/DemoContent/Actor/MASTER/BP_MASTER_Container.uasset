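; BP_MASTER_Container is a master container actor that opens and closes a container screen when interacted with.
; On BeginPlay it creates and caches a WB_ContainerScreen widget and passes itself to it as ContainerRef.
; OnInteract toggles on the widget's visibility, adding or removing it with a sound and switching cursor and input mode.
; It also pauses or resumes the game and disables or enables the BP_IMPPlayer HUD.
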(event EventBeginPlay
  (if (not (Utilities|IsValid (Variables|Default|GetContainerScreenRef)))
    (bind _returnvalue (UserInterface|CreateWidget (Variables|Default|GetOpenContainerScreen)))
    (bind _aswb_container_screen (Utilities|Casting|CastToWB_ContainerScreen _returnvalue))
    (bind _output_get (Variables|Default|SetContainerScreenRef _aswb_container_screen))
    (Variables|/Game/DemoContent/UI/WB_ContainerScreen.WB_ContainerScreen_C|SetContainerRef _output_get self)))

(event Collision|EventActorBeginOverlap
  (params (OtherActor :type Actor%20Object%20Reference)))

(event EventTick
  (params (DeltaSeconds :type Float%20%28single-precision%29)))

(event EventOnInteract
  (bind _returnvalue (Game|GetPlayerController 0))
  (if (Widget|IsVisible (Variables|Default|GetContainerScreenRef))
    (Widget|RemovefromParent (Variables|Default|GetContainerScreenRef))
    (Audio|PlaySound2D (Variables|Default|GetClosingSound) 1.0 1.0 0.0 0 0)
    (Variables|/Script/Engine.PlayerController|SetbShowMouseCursor _returnvalue false)
    (Input|SetInputModeGameOnly _returnvalue)
    (bind _asbp_impplayer (Utilities|Casting|CastToBP_IMPPlayer (Game|Player|GetPlayerPawn 0)))
    (Default|EnableHUD _asbp_impplayer)
    (Game|SetGamePaused false)
    (else
      (Audio|PlaySound2D (Variables|Default|GetOpenSound) 1.0 1.0 0.0 0 0)
      (UserInterface|Viewport|AddtoViewport (Variables|Default|GetContainerScreenRef) 0)
      (Variables|/Script/Engine.PlayerController|SetbShowMouseCursor _returnvalue true)
      (Input|SetInputModeGameandUI _returnvalue (Variables|Default|GetContainerScreenRef) "DoNotLock" true)
      (bind _asbp_impplayer_2 (Utilities|Casting|CastToBP_IMPPlayer (Game|Player|GetPlayerPawn 0)))
      (Default|DisableHUD _asbp_impplayer_2)
      (Game|SetGamePaused true))))

(fn ConstructionScript)