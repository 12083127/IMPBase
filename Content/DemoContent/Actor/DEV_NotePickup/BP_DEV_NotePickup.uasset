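; BP_DEV_NotePickup is a demo interactable note pickup that adds a note to the player's journal and shows it on screen.
; On interact, it runs the parent logic, plays a paper sound and looks up the entry matching its NoteID through the IMP player state.
; That entry is added to the journal, and its body text fills a newly created note widget on the viewport.
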(event EventBeginPlay)

(event Collision|EventActorBeginOverlap
  (params (OtherActor :type Actor%20Object%20Reference)))

(event EventTick
  (params (DeltaSeconds :type Float%20%28single-precision%29)))

(event EventOnInteract
  (|CallParentFunction)
  (bind _asimpplayer (Utilities|Casting|CastToIMPPlayer (Game|Player|GetPlayerPawn 0)))
  (Variables|Default|SetPlayer _asimpplayer)
  (Audio|PlaySoundatLocation "/Game/DemoContent/Actor/DEV_NotePickup/NotePickup_dev/PaperSoundEffect.PaperSoundEffect" (Transformation|GetActorLocation) "0, 0, 0" 1.0 1.0 0.0 0 0 0)
  (bind _asimpplayer_state (Utilities|Casting|CastToIMPPlayerState (Variables|/Script/Engine.Pawn|GetPlayerState (Variables|Default|GetPlayer))))
  (Class|IMPPlayerState|AddNotetoPlayerJournal _asimpplayer_state (Class|IMPPlayerState|FindNoteEntry _asimpplayer_state (Variables|Default|GetNoteID)))
  (bind _returnvalue (UserInterface|CreateWidget "/Game/DemoContent/Actor/DEV_NotePickup/NotePickup_dev/NoteWidget.NoteWidget_C"))
  (UserInterface|Viewport|AddtoViewport _returnvalue 0)
  (Rendering|Components|TextRender|SetText (Variables|/Game/DemoContent/Actor/DEV_NotePickup/NotePickup_dev/NoteWidget.NoteWidget_C|GetNote_Body _returnvalue) (.NoteBody (Utilities|Struct|BreakIMPNoteEntry (Class|IMPPlayerState|FindNoteEntry _asimpplayer_state (Variables|Default|GetNoteID))))))

(fn ConstructionScript)