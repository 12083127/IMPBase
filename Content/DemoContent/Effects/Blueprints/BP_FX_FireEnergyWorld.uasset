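; BP_FX_FireEnergyWorld is a timed fire hazard in the world that applies a fire debuff to NPC characters.
; On begin play it schedules a decal fade-out based on Duration, which also destroys the actor when finished.
; Overlapping BP_MASTER_IMPNPCCharacterBase actors receive the debuff only while more than one second of Duration remains.
; Tick counts Duration down and deactivates the Fire component at zero.
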(event EventBeginPlay
  (bind _duration (Variables|Default|GetDuration))
  (Rendering|Components|Decal|SetFadeOut (Variables|Default|GetDecal) (- _duration 1.0) (+ _duration 2.0) true))

(event Collision|EventActorBeginOverlap
  (params (OtherActor :type Actor%20Object%20Reference))
  (if (> (Variables|Default|GetDuration) 1.0)
    (bind _asbp_master_impnpccharacter_base (Utilities|Casting|CastToBP_MASTER_IMPNPCCharacterBase OtherActor))
    (Default|ApplyFireDebuff _asbp_master_impnpccharacter_base (Variables|Default|GetFireDamagePerSec) "0, 0, 0")))

(event EventTick
  (params (DeltaSeconds :type Float%20%28single-precision%29))
  (bind _output_get (Variables|Default|SetDuration (Math|Float|Clamp(Float) (- (Variables|Default|GetDuration) DeltaSeconds) 0.0 (Variables|Default|GetDuration))))
  (if (<= _output_get 0.0)
    (Components|Activation|SetActive (Variables|Default|GetFire) false false)))

(fn ConstructionScript)