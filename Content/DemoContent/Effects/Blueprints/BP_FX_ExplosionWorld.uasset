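; BP_FX_ExplosionWorld is a short-lived explosion volume that damages NPC characters caught inside it.
; Any overlapping actor derived from BP_MASTER_IMPNPCCharacterBase receives ApplyExplosionDamage from the explosion's location, with force set to a third of the damage.
; Tick uses frame-length delays to switch off the Sphere's overlap events and then destroy the actor, limiting hits to a brief window after spawn.
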(event EventBeginPlay)

(event EventTick
  (params (DeltaSeconds :type Float%20%28single-precision%29))
  (Utilities|FlowControl|Delay DeltaSeconds)
  (Variables|/Script/Engine.PrimitiveComponent|SetbGenerateOverlapEvents (Variables|Default|GetSphere) false)
  (Utilities|FlowControl|Delay DeltaSeconds)
  (Actor|DestroyActor))

(event Collision|EventActorBeginOverlap
  (params (OtherActor :type Actor%20Object%20Reference))
  (bind _asbp_master_impnpccharacter_base (Utilities|Casting|CastToBP_MASTER_IMPNPCCharacterBase OtherActor))
  (Default|ApplyExplosionDamage _asbp_master_impnpccharacter_base (Variables|Default|GetExplosionDamage) (Transformation|GetActorLocation) (Math|Float|SafeDivide (Variables|Default|GetExplosionDamage) 3.0)))

(fn ConstructionScript)