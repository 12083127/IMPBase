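; BP_FX_SmokeScreenWorld is a world-placed smoke screen effect that blinds NPCs touching it.
; On overlap, any IMP NPC character other than BP_IMPEnemy_Water01 has its CanSeePlayer blackboard key set false, with a debug print.
; Tick grows the smoke's world scale up to a clamp and counts down Duration, then deactivates the effect and destroys the actor after a delay.
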(event EventBeginPlay)

(event Collision|EventActorBeginOverlap
  (params (OtherActor :type Actor%20Object%20Reference))
  (bind _asbp_master_impnpccharacter_base (Utilities|Casting|CastToBP_MASTER_IMPNPCCharacterBase OtherActor))
  (if (!= _asbp_master_impnpccharacter_base "/Game/DemoContent/Pawn/NPCCharacterBase/BP_IMPEnemy_Water01.BP_IMPEnemy_Water01")
    (AI|Components|Blackboard|SetValueasBool (AI|GetBlackboard _asbp_master_impnpccharacter_base) (Utilities|Name|MakeLiteralName "CanSeePlayer") false)
    (Development|PrintString "I CANT SEE")))

(event EventTick
  (params (DeltaSeconds :type Float%20%28single-precision%29))
  (bind _output_get (Variables|Default|SetScale (Math|Vector|ClampVectorSize (+ (Variables|Default|GetScale) (Math|Interpolation|FInterpTo 0.0 0.5 DeltaSeconds 1.0)) 0.0 3.0)))
  (Transformation|SetWorldScale3D (Variables|Default|GetSmokeScreen) _output_get)
  (bind _output_get_2 (Variables|Default|SetDuration (Math|Float|Clamp(Float) (- (Variables|Default|GetDuration) DeltaSeconds) 0.0 (Variables|Default|GetDuration))))
  (if (<= _output_get_2 0.0)
    (Components|Activation|SetActive (Variables|Default|GetSmokeScreen) false false)
    (Utilities|FlowControl|Delay 7.0)
    (Actor|DestroyActor)))

(fn ConstructionScript)