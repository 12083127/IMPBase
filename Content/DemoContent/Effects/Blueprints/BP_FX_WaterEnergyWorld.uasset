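; BP_FX_WaterEnergyWorld is a water-energy effect actor with a decal that cleans itself up.
; On BeginPlay it schedules the decal fade-out with start delay and fade length derived from Duration, destroying the actor when the fade completes.
; Tick and overlap events are empty, and a leftover Duration countdown is disconnected and never runs.
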(event EventBeginPlay
  (bind _duration (Variables|Default|GetDuration))
  (Rendering|Components|Decal|SetFadeOut (Variables|Default|GetDecal) (- _duration 1.0) (+ _duration 3.0) true))

(event Collision|EventActorBeginOverlap
  (params (OtherActor :type Actor%20Object%20Reference)))

(event EventTick
  (params (DeltaSeconds :type Float%20%28single-precision%29)))

(fn ConstructionScript)