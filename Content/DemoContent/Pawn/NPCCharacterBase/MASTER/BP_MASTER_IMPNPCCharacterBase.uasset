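; Master NPC character Blueprint that drives an energy-themed aura and implements explosion, fire and paralysis effects.
; The construction script picks an aura color from the EnergyComponent's type, BeginPlay applies it to mesh materials, and Tick feeds in normalized energy level.
; Explosions deal damage and push the mesh bodies away from impact.
; Fire attaches particles at the nearest bone or pelvis and stores damage per second, while paralysis sets a Blackboard flag.
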(event EventBeginPlay
  (|CallParentFunction)
  (Rendering|Material|SetVectorParameterValueonMaterials (Variables|Character|GetMesh) "AuraColor" (Math|Conversions|ToVector(LinearColor) (Variables|Default|GetNewAuraColor))))

(event Collision|EventActorBeginOverlap
  (params (OtherActor :type Actor%20Object%20Reference)))

(event EventTick
  (params (DeltaSeconds :type Float%20%28single-precision%29))
  (|CallParentFunction DeltaSeconds)
  (Rendering|Material|SetScalarParameterValueonMaterials (Variables|Character|GetMesh) "EnergyLevel" (Class|IMPEnergyComponent|GetEnergyLevelNormalized (Variables|Default|GetEnergyComponent))))

(fn ConstructionScript
  (bind _energycolorstruct (LocalVariables|GetEnergyColorStruct))
  (switch Utilities|FlowControl|Switch|SwitchonEEnergyType (Class|IMPEnergyComponent|GetEnergyType (Variables|Default|GetEnergyComponent))
    (:ET_Electric
      (Variables|Default|SetNewAuraColor (.electricenergycolor _energycolorstruct)))
    (:ET_Fire
      (Variables|Default|SetNewAuraColor (.fireenergycolor _energycolorstruct)))
    (:ET_Water
      (Variables|Default|SetNewAuraColor (.waterenergycolor _energycolorstruct)))))

(fn ApplyExplosionDamage
  (params (Damage :type Float%20%28single-precision%29) (ImpactLocation :type Vector) (Force :type Float%20%28single-precision%29))
  (bind _mesh (Variables|Character|GetMesh))
  (if (not (Class|IMPNPCCharacterBase|IsDead))
    (Class|IMPNPCCharacterBase|DamageNPC Damage "0, 0, 0")
    (Class|SkeletalMeshComponent|AddImpulsetoAllBodiesBelow _mesh (* (- (Transformation|GetWorldLocation _mesh) ImpactLocation) Force) "None" false true)))

(fn ApplyFireDebuff
  (params (DamagePerSecond :type Float%20%28single-precision%29) (ImpactLocation :type Vector))
  (bind _fxfiredebuff (Variables|Default|GetFXFireDebuff))
  (bind _mesh (Variables|Character|GetMesh))
  (if (and (not (Class|IMPNPCCharacterBase|IsDead)) (not (Variables|Default|GetbBurning)))
    (Variables|Default|SetbBurning true)
    (if (Math|Vector|Equal(Vector) ImpactLocation "0, 0, 0" 0.0001)
      (bind _returnvalue (Effects|SpawnEmitterAttached _fxfiredebuff _mesh "pelvis"))
      (Variables|Default|SetPSFireDebuff _returnvalue)
      (else
        (bind _returnvalue_2 (Effects|SpawnEmitterAttached _fxfiredebuff _mesh (.ReturnValue (Class|SkinnedMeshComponent|FindClosestBoneK2 _mesh ImpactLocation 0.0))))
        (Variables|Default|SetPSFireDebuff _returnvalue_2)))
    (Variables|Default|SetFireDamagePerSec DamagePerSecond)))

(fn ApplyParalyzeEffect
  (bind _returnvalue (Utilities|Name|MakeLiteralName "IsParalyzed"))
  (bind _self self)
  (bind _returnvalue_2 (AI|GetBlackboard _self))
  (if (and (not (Class|IMPNPCCharacterBase|IsDead)) (not (ScalableFloat|GetValueasBool _returnvalue_2 _returnvalue)))
    (AI|Components|Blackboard|SetValueasBool _returnvalue_2 _returnvalue true)))