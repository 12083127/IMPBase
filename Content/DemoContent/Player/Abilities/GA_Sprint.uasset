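; Gameplay ability that runs player sprinting.
; Activation applies the GE_SprintTags effect and sets walk speed from the player's GetMaxSpeed.
; It commits its cost every 0.1 seconds while sprinting, ending on input release or failed commit.
; Ending removes the effect, clears the sprint flag and refreshes speed, using player pawn 0 rather than the ability owner.
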(event Ability|EventActivateAbility
  (bind _returnvalue (Ability|GetActorInfo))
  (bind _returnvalue_2 (Ability|ApplyGameplayEffectToOwner "/Game/DemoContent/Player/Abilities/GE_SprintTags.GE_SprintTags_C"))
  (Variables|Default|SetGESprintTags _returnvalue_2)
  (bind _ascharacter_movement_component (Utilities|Casting|CastToCharacterMovementComponent (.movementcomponent _returnvalue)))
  (Variables|/Script/Engine.CharacterMovementComponent|SetMaxWalkSpeed _ascharacter_movement_component (Class|IMPPlayer|GetMaxSpeed (.AsIMPPlayer (Utilities|Casting|CastToIMPPlayer (.owneractor _returnvalue)))))
  (Ability|Tasks|WaitInputRelease true
    (:then
      (bind _returnvalue_3 (Ability|CommitAbilityCost false :!label _label))
      (if _returnvalue_3
        (if (Class|IMPPlayer|IsSprinting (.AsIMPPlayer (Utilities|Casting|CastToIMPPlayer (Game|Player|GetPlayerPawn 0))))
          (Ability|Tasks|WaitDelay 0.1
            (:OnFinish
              (goto _label))))
        (else
          (Ability|EndAbility :!label _label_2))))
    (:OnRelease
      (goto _label_2))))

(event Ability|EventOnEndAbility
  (params (bWasCancelled :type Boolean))
  (bind _returnvalue (Game|Player|GetPlayerPawn 0))
  (bind _asimpplayer (Utilities|Casting|CastToIMPPlayer _returnvalue))
  (Ability|RemoveGameplayEffectFromOwnerWithHandle (Variables|Default|GetGESprintTags))
  (Class|IMPPlayer|SetIsSprinting _asimpplayer false)
  (bind _ascharacter_movement_component (Utilities|Casting|CastToCharacterMovementComponent (Pawn|GetMovementComponent _asimpplayer)))
  (Variables|/Script/Engine.CharacterMovementComponent|SetMaxWalkSpeed _ascharacter_movement_component (Class|IMPPlayer|GetMaxSpeed _asimpplayer)))