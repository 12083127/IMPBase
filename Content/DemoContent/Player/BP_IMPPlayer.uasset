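; Player character Blueprint for an elemental shooter, layering fire, water and electric combat and UI onto its parent class.
; Tick drives element indicator materials, while imbued lethal shots burn, paralyze or detonate burning NPCs.
; Energy shots trace from the camera to spawn element actors, combining fire and water into smoke, electric and fire into explosions, electric and water into paralysis.
; Input toggles HUD, pausing inventory, journal and test menu, plus debug item and enemy spawning.
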(event EventBeginPlay
  (|CallParentFunction)
  (CallFunction|EnableHUD))

(event Collision|EventActorBeginOverlap
  (params (OtherActor :type Actor%20Object%20Reference)))

(event EventTick
  (params (DeltaSeconds :type Float%20%28single-precision%29))
  (bind _activeelementindicator (Variables|Default|GetActiveElementIndicator))
  (bind _activeelementindicator_2 (Variables|Default|GetActiveElementIndicator))
  (|CallParentFunction DeltaSeconds)
  (bind _returnvalue (Class|IMPPlayer|GetEnergyLevelNormalized "ET_Fire"))
  (Rendering|Material|SetScalarParameterValueonMaterials (Variables|Default|GetFireElementIndicator) "EnergyLevel" _returnvalue)
  (bind _returnvalue_2 (Class|IMPPlayer|GetEnergyLevelNormalized "ET_Water"))
  (Rendering|Material|SetScalarParameterValueonMaterials (Variables|Default|GetWaterElementIndicator) "EnergyLevel" _returnvalue_2)
  (bind _returnvalue_3 (Class|IMPPlayer|GetEnergyLevelNormalized "ET_Electric"))
  (Rendering|Material|SetScalarParameterValueonMaterials (Variables|Default|GetElectricElementIndicator) "EnergyLevel" _returnvalue_3)
  (switch Utilities|FlowControl|Switch|SwitchonEEnergyType (Class|IMPPlayer|GetActiveElement)
    (:ET_Electric
      (Rendering|Material|SetMaterial _activeelementindicator_2 0 "/Game/DemoContent/Materials/M_EnergyBarElectric_01.M_EnergyBarElectric_01"))
    (:ET_Fire
      (Rendering|Material|SetMaterial _activeelementindicator_2 0 "/Game/DemoContent/Materials/M_EnergyBarFire_01.M_EnergyBarFire_01"))
    (:ET_Water
      (Rendering|Material|SetMaterial _activeelementindicator_2 0 "/Game/DemoContent/Materials/M_EnergyBarWater_01.M_EnergyBarWater_01")))
  (if (== (Class|IMPPlayer|GetCurrentMode) 0)
    (Rendering|Material|SetScalarParameterValueonMaterials _activeelementindicator "EnergyLevel" 1.0)
    (elif (and (Class|IMPPlayer|UsesImbuement) (Class|IMPPlayer|HasActiveElementEnergy))
      (Rendering|Material|SetScalarParameterValueonMaterials _activeelementindicator "EnergyLevel" 0.5)
      (else
        (Rendering|Material|SetScalarParameterValueonMaterials _activeelementindicator "EnergyLevel" 0.0)))))

(event EventOnShootEnergy
  (params (DeltaTime :type Float%20%28single-precision%29))
  (bind _followcamera (Variables|Default|GetFollowCamera))
  (bind _returnvalue (Transformation|GetWorldLocation _followcamera))
  (|CallParentFunction DeltaTime)
  (Utilities|FlowControl|Delay 0.1) ; hacky delay to avoid one 90 degree offshot line trace that mysteriously occurs. This should be removed after fixing the issue
  (bind (_outhit _returnvalue_2) (Collision|LineTraceByChannel _returnvalue (+ _returnvalue (* (Math|Vector|GetForwardVector _followcamera) 1.5e+03)) "TraceTypeQuery2" false 0 "None"))
  (if _returnvalue_2
    (Variables|Default|SetImpactLoc (.Location (Collision|BreakHitResult _outhit)))
    (Variables|Default|SetImpactNormal (.ImpactNormal (Collision|BreakHitResult _outhit)))
    (switch Utilities|FlowControl|Switch|SwitchonEEnergyType (Class|IMPPlayer|GetActiveElement)
      (:ET_Electric
        ;[1 1 1] Check for active Fire, if Y -> kill fire and replace with explosion
        (bind _asbp_fx_fire_energy_world (Utilities|Casting|CastToBP_FX_FireEnergyWorld (.HitActor (Collision|BreakHitResult _outhit)))
          (:then
            (if (> (Variables|/Game/DemoContent/Effects/Blueprints/BP_FX_FireEnergyWorld.BP_FX_FireEnergyWorld_C|GetDuration _asbp_fx_fire_energy_world) 0.0)
              (bind _outactors (Collision|SphereOverlapActors (Transformation|GetActorLocation _asbp_fx_fire_energy_world) 72.0 (Utilities|Array|MakeArray "ObjectTypeQuery2") "/Game/DemoContent/Effects/Blueprints/BP_FX_FireEnergyWorld.BP_FX_FireEnergyWorld_C"))
              (for _array_element _outactors
                (bind _asbp_fx_fire_energy_world_2 (Utilities|Casting|CastToBP_FX_FireEnergyWorld _array_element))
                (Variables|/Game/DemoContent/Effects/Blueprints/BP_FX_FireEnergyWorld.BP_FX_FireEnergyWorld_C|SetDuration _asbp_fx_fire_energy_world_2 0.0)
                (Rendering|Components|Decal|SetFadeOut (Variables|/Game/DemoContent/Effects/Blueprints/BP_FX_FireEnergyWorld.BP_FX_FireEnergyWorld_C|GetDecal _asbp_fx_fire_energy_world_2) 0.0 3.0 true))
              (Game|SpawnActorfromClass "/Game/DemoContent/Effects/Blueprints/BP_FX_ExplosionWorld.BP_FX_ExplosionWorld_C" (Math|Conversions|ToTransform(Vector) (Transformation|GetActorLocation _asbp_fx_fire_energy_world)) "Undefined" 0 0)
              ;[1 1 1] Spawn Electric
              (bind _returnvalue_3 (Collision|SphereOverlapActors (Variables|Default|GetImpactLoc) 32.0 (Utilities|Array|MakeArray "ObjectTypeQuery2") "/Game/DemoContent/Effects/Blueprints/BP_FX_ElectricEnergyWorld.BP_FX_ElectricEnergyWorld_C" :!label _label))
              (if (not _returnvalue_3)
                (Game|SpawnActorfromClass "/Game/DemoContent/Effects/Blueprints/BP_FX_ElectricEnergyWorld.BP_FX_ElectricEnergyWorld_C" (Math|Conversions|ToTransform(Vector) (Variables|Default|GetImpactLoc)) "Undefined" 0 0))
              (else
                ;[1 1 1] Check for active Water, if Y -> kill Water and replace with paralyze
                (bind _asbp_fx_water_energy_world (Utilities|Casting|CastToBP_FX_WaterEnergyWorld (.HitActor (Collision|BreakHitResult _outhit)) :!label _label_2)
                  (:then
                    (if (> (Variables|/Game/DemoContent/Effects/Blueprints/BP_FX_WaterEnergyWorld.BP_FX_WaterEnergyWorld_C|GetDuration _asbp_fx_water_energy_world) 0.0)
                      (bind _outactors_2 (Collision|SphereOverlapActors (Transformation|GetActorLocation _asbp_fx_water_energy_world) 96.0 (Utilities|Array|MakeArray "ObjectTypeQuery2") "/Game/DemoContent/Effects/Blueprints/BP_FX_WaterEnergyWorld.BP_FX_WaterEnergyWorld_C"))
                      (for _array_element_2 _outactors_2
                        (bind _asbp_fx_water_energy_world_2 (Utilities|Casting|CastToBP_FX_WaterEnergyWorld _array_element_2))
                        (Variables|/Game/DemoContent/Effects/Blueprints/BP_FX_WaterEnergyWorld.BP_FX_WaterEnergyWorld_C|SetDuration _asbp_fx_water_energy_world_2 0.0)
                        (Rendering|Components|Decal|SetFadeOut (Variables|/Game/DemoContent/Effects/Blueprints/BP_FX_WaterEnergyWorld.BP_FX_WaterEnergyWorld_C|GetDecal _asbp_fx_water_energy_world_2) 0.0 2.0 true))
                      (Game|SpawnActorfromClass "/Game/DemoContent/Effects/Blueprints/BP_FX_ParalyzeEffectWorld.BP_FX_ParalyzeEffectWorld_C" (Math|Conversions|ToTransform(Vector) (Transformation|GetActorLocation _asbp_fx_water_energy_world)) "Undefined" 0 0)))
                  (:CastFailed
                    (goto _label))))))
          (:CastFailed
            (goto _label_2))))
      (:ET_Fire
        ;[1 1 1] Spawn Fire
        (bind _returnvalue_4 (Collision|SphereOverlapActors (Variables|Default|GetImpactLoc) 16.0 (Utilities|Array|MakeArray "ObjectTypeQuery2") 0))
        (if (not _returnvalue_4)
          (Game|SpawnActorfromClass "/Game/DemoContent/Effects/Blueprints/BP_FX_FireEnergyWorld.BP_FX_FireEnergyWorld_C" (Math|Conversions|ToTransform(Vector) (Variables|Default|GetImpactLoc)) "Undefined" 0 0)))
      (:ET_Water
        ;[1 1 1] Check for active Fire, if Y -> kill fire and replace with smokescreen
        (bind _asbp_fx_fire_energy_world_3 (Utilities|Casting|CastToBP_FX_FireEnergyWorld (.HitActor (Collision|BreakHitResult _outhit)))
          (:then
            (if (> (Variables|/Game/DemoContent/Effects/Blueprints/BP_FX_FireEnergyWorld.BP_FX_FireEnergyWorld_C|GetDuration _asbp_fx_fire_energy_world_3) 0.0)
              (bind _outactors_3 (Collision|SphereOverlapActors (Transformation|GetActorLocation _asbp_fx_fire_energy_world_3) 72.0 (Utilities|Array|MakeArray "ObjectTypeQuery2") "/Game/DemoContent/Effects/Blueprints/BP_FX_FireEnergyWorld.BP_FX_FireEnergyWorld_C"))
              (for _array_element_3 _outactors_3
                (bind _asbp_fx_fire_energy_world_4 (Utilities|Casting|CastToBP_FX_FireEnergyWorld _array_element_3))
                (Variables|/Game/DemoContent/Effects/Blueprints/BP_FX_FireEnergyWorld.BP_FX_FireEnergyWorld_C|SetDuration _asbp_fx_fire_energy_world_4 0.0)
                (Rendering|Components|Decal|SetFadeOut (Variables|/Game/DemoContent/Effects/Blueprints/BP_FX_FireEnergyWorld.BP_FX_FireEnergyWorld_C|GetDecal _asbp_fx_fire_energy_world_4) 0.0 3.0 true))
              (bind _returnvalue_5 (Collision|SphereOverlapActors (Transformation|GetActorLocation _asbp_fx_fire_energy_world_3) 72.0 (Utilities|Array|MakeArray "ObjectTypeQuery2") "/Game/DemoContent/Effects/Blueprints/BP_FX_SmokeScreenWorld.BP_FX_SmokeScreenWorld_C"))
              (if (not _returnvalue_5)
                (Game|SpawnActorfromClass "/Game/DemoContent/Effects/Blueprints/BP_FX_SmokeScreenWorld.BP_FX_SmokeScreenWorld_C" (Math|Conversions|ToTransform(Vector) (Transformation|GetActorLocation _asbp_fx_fire_energy_world_3)) "Undefined" 0 0))
              (else
                ;[1 1 1] Spawn Water
                (bind _returnvalue_6 (Collision|SphereOverlapActors (Variables|Default|GetImpactLoc) 16.0 (Utilities|Array|MakeArray "ObjectTypeQuery2") "/Game/DemoContent/Effects/Blueprints/BP_FX_WaterEnergyWorld.BP_FX_WaterEnergyWorld_C" :!label _label_3))
                (if (not _returnvalue_6)
                  (Game|SpawnActorfromClass "/Game/DemoContent/Effects/Blueprints/BP_FX_WaterEnergyWorld.BP_FX_WaterEnergyWorld_C" (Math|Conversions|ToTransform(Vector) (Variables|Default|GetImpactLoc)) "Undefined" 0 0)))))
          (:CastFailed
            (goto _label_3)))))))

(event EventOnShootLethal
  (bind _shotactor (Variables|Default|GetShotActor))
  (|CallParentFunction)
  (if (and (Class|IMPPlayer|HasActiveElementEnergy) (Class|IMPPlayer|UsesImbuement))
    (bind _asbp_master_impnpccharacter_base (Utilities|Casting|CastToBP_MASTER_IMPNPCCharacterBase (.hitactor _shotactor))
      (:then
        (Variables|Default|SetShotNPC _asbp_master_impnpccharacter_base)
        (switch Utilities|FlowControl|Switch|SwitchonEEnergyType (Class|IMPPlayer|GetActiveElement)
          (:ET_Electric
            (if (Variables|/Game/DemoContent/Pawn/NPCCharacterBase/MASTER/BP_MASTER_IMPNPCCharacterBase.BP_MASTER_IMPNPCCharacterBase_C|GetbBurning (Variables|Default|GetShotNPC))
              (Default|ApplyExplosionDamage (Variables|Default|GetShotNPC) 1e+02 (- (Transformation|GetActorLocation (Variables|Default|GetShotNPC)) (* (Math|Vector|GetUnitDirection(Vector) (.tracestart _shotactor) (.impactpoint _shotactor)) 1e+02)) 25.0)
              (Effects|SpawnEmitteratLocation "/Game/StarterContent/Particles/P_Explosion.P_Explosion" (.impactpoint _shotactor) "0, 0, 0" "0.500000,0.500000,0.500000")
              (else
                (Default|ApplyParalyzeEffect (Variables|Default|GetShotNPC))
                (Effects|SpawnEmitteratLocation "/Game/DemoContent/Effects/ParticleSystems/P_IMPParalyzeEffectWorld.P_IMPParalyzeEffectWorld" "0, 0, 0" "0, 0, 0" "0.100000,0.100000,0.100000"))))
          (:ET_Fire
            (Default|ApplyFireDebuff (Variables|Default|GetShotNPC) 1e+01 (.impactpoint _shotactor)))))
      (:CastFailed
        (Variables|Default|SetShotNPC 0)))))

(event Input|ActionEvents|InputActionCharMenu
  (params (Key :type Key%20Structure :default "None"))
  (bind _returnvalue (Game|GetPlayerController 0))
  (:Pressed
    (if (Utilities|IsValid (Variables|Default|GetInventoryScreen))
      _
      (else
        (bind _returnvalue_2 (UserInterface|CreateWidget "/Game/DemoContent/UI/Inventory/WB_InventoryScreen.WB_InventoryScreen_C" (Game|GetPlayerController 0)))
        (Variables|Default|SetInventoryScreen _returnvalue_2)))
    (if (Widget|IsVisible (Variables|Default|GetIngameHUD))
      (CallFunction|DisableHUD)
      (UserInterface|Viewport|AddtoViewport (Variables|Default|GetInventoryScreen) 0)
      (Variables|/Script/Engine.PlayerController|SetbShowMouseCursor _returnvalue true)
      (Input|SetInputModeGameandUI _returnvalue (Variables|Default|GetInventoryScreen) "DoNotLock" false)
      (Game|SetGamePaused true)
      (elif (Widget|IsVisible (Variables|Default|GetInventoryScreen))
        (Widget|RemovefromParent (Variables|Default|GetInventoryScreen))
        (CallFunction|EnableHUD)
        (Variables|/Script/Engine.PlayerController|SetbShowMouseCursor _returnvalue false)
        (Input|SetInputModeGameOnly _returnvalue)
        (Game|SetGamePaused false)))))

(event Input|ActionEvents|InputActionAI_Sprint
  (params (Key :type Key%20Structure :default "None")))

(event Input|KeyboardEvents|J
  (params (Key :type Key%20Structure :default "None"))
  (bind _returnvalue (Game|GetPlayerController 0))
  (:Pressed
    (if (Utilities|IsValid (Variables|Default|GetJournalScreen))
      (Widget|RemovefromParent (Variables|Default|GetJournalScreen))
      (Variables|Default|SetJournalScreen 0)
      (Input|SetInputModeGameOnly _returnvalue)
      (Variables|/Script/Engine.PlayerController|SetbShowMouseCursor _returnvalue false)
      (else
        (bind _returnvalue_2 (UserInterface|CreateWidget "/Game/DemoContent/UI/WB_JournalScreen.WB_JournalScreen_C" (Game|GetPlayerController 0)))
        (bind _output_get (Variables|Default|SetJournalScreen _returnvalue_2))
        (UserInterface|Viewport|AddtoViewport _output_get 0)
        (Input|SetInputModeGameandUI _returnvalue _output_get "DoNotLock" true)
        (Variables|/Script/Engine.PlayerController|SetbShowMouseCursor _returnvalue true)))))

(event Input|KeyboardEvents|Ö
  (params (Key :type Key%20Structure :default "None"))
  (bind _returnvalue (Game|GetPlayerController 0))
  (:Pressed
    (if (Utilities|IsValid (Variables|Default|GetMainTest))
      _
      (else
        (bind _returnvalue_2 (UserInterface|CreateWidget "/Game/DemoContent/UI/TEST/WB_Main.WB_Main_C" (Game|GetPlayerController 0)))
        (Variables|Default|SetMainTest _returnvalue_2)))
    (if (Widget|IsVisible (Variables|Default|GetMainTest))
      (Widget|RemovefromParent (Variables|Default|GetMainTest))
      (Variables|/Script/Engine.PlayerController|SetbShowMouseCursor _returnvalue false)
      (Input|SetInputModeGameOnly _returnvalue)
      (else
        (UserInterface|Viewport|AddtoViewport (Variables|Default|GetMainTest) 0)
        (Variables|/Script/Engine.PlayerController|SetbShowMouseCursor _returnvalue true)
        (Input|SetInputModeGameandUI _returnvalue (Variables|Default|GetMainTest) "DoNotLock" false)))))

(event Input|MouseEvents|ThumbMouseButton2
  (params (Key :type Key%20Structure :default "None"))
  (bind _followcamera (Variables|Default|GetFollowCamera))
  (bind _returnvalue (Transformation|GetWorldLocation _followcamera))
  ;[1 1 1] DEBUGGING: Spawn NPCs for testing
  (:Released
    (bind (_outhit _returnvalue_2) (Collision|LineTraceByChannel _returnvalue (+ _returnvalue (* (Math|Vector|GetForwardVector _followcamera) 3e+03)) "TraceTypeQuery2" false 0 "None"))
    (if _returnvalue_2
      (AI|SpawnAIFromClass "/Game/DemoContent/Pawn/NPCCharacterBase/BP_IMPEnemy_Fire01.BP_IMPEnemy_Fire01_C" 0 (.Location (Collision|BreakHitResult _outhit)) "0, 0, 0" false 0))))

(event Input|KeyboardEvents|U
  (params (Key :type Key%20Structure :default "None"))
  (bind _inventory (Variables|Default|GetInventory))
  (:Pressed
    (Class|IMPInventoryComponent|RemoveItem _inventory (Class|IMPInventoryComponent|FindItem _inventory "/Game/DemoContent/Items/BP_Item_Food_001.BP_Item_Food_001_C") true)))

(event Input|KeyboardEvents|+
  (params (Key :type Key%20Structure :default "None"))
  (:Pressed
    (Class|IMPInventoryComponent|AddItembyClass (Variables|Default|GetInventory) "/Game/DemoContent/Items/BP_Item_Food_001.BP_Item_Food_001_C")))

(fn ConstructionScript)

(fn EnableHUD
  (if (Utilities|IsValid (Variables|Default|GetIngameHUD))
    _
    (else
      (bind _returnvalue (UserInterface|CreateWidget "/Game/DemoContent/UI/WB_HUD_Ingame.WB_HUD_Ingame_C" (Game|GetPlayerController 0)))
      (Variables|Default|SetIngameHUD _returnvalue)))
  (UserInterface|Viewport|AddtoViewport (Variables|Default|GetIngameHUD) 0))

(fn DisableHUD
  (Widget|RemovefromParent (Variables|Default|GetIngameHUD)))

(fn GetSkeletalMeshComponent
  (return (Variables|Character|GetMesh)))